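; BP_HearthParent is a parent actor with a sphere component and a gravity value, apparently an early prototype of gravity acting on the player.
; BeginPlay caches the third-person player character.
; Each Tick line-traces from the character's mesh, using the mesh-to-sphere offset scaled by GravitéA1 over 9.81 directly as the world-space end point.
; The trace only draws persistent debug lines; its result is unused and no force is applied.
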(event `self.ReceiveBeginPlay`
  (bind _asbp_third_person_character (cast `/Game/ThirdPerson/Blueprints/BP_ThirdPersonCharacter` (`GameplayStatics.GetPlayerCharacter` 0)))
  (set `self.As BP Third Person Character` _asbp_third_person_character))

(event `self.ReceiveTick`
  (params (DeltaSeconds :type "Float (single-precision)"))
  (bind _returnvalue (`SceneComponent.K2_GetComponentLocation` (`Character.Mesh` (`self.As BP Third Person Character`))))
  (`KismetSystemLibrary.LineTraceSingle` :`Start` _returnvalue :`End` (* (- (`SceneComponent.K2_GetComponentLocation` (`self.Sphere`)) _returnvalue) (/ (`self.Gravité_A1`) 9.81)) :`TraceChannel` "TraceTypeQuery1" :`DrawDebugType` "Persistent"))

(fn `UserConstructionScript`)